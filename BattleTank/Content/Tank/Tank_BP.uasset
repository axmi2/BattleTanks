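; Player-controllable tank Blueprint that wires its track, turret and barrel components into movement and aiming components on BeginPlay.
; Camera input rotates an azimuth gimbal for yaw and a spring arm for pitch, while Fire triggers the aiming component.
; Driving supports both direct per-track throttle and forward/turn intent axes routed through the movement component.
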(event `self.ReceiveBeginPlay`
  (`TankMovementComponent.Initialise` (`self.TankMovement`) (`self.TankTrack_L`) (`self.TankTrack_R`))
  (`TankAimingComponent.Initialise_Aiming` (`self.TankAiming`) (`self.TankBarrel`) (`self.TankTurret`)))

(event `InputAxis|AimAzimuth`
  (params (AxisValue :type "Float (single-precision)"))
  (`SceneComponent.K2_AddLocalRotation` (`self.AzimuthGimbal`) (`KismetMathLibrary.MakeRotator` 0.0 0.0 AxisValue) false false))

(event `InputAxis|AimElevation`
  (params (AxisValue :type "Float (single-precision)"))
  (`SceneComponent.K2_AddLocalRotation` (`self.SpringArm`) (`KismetMathLibrary.MakeRotator` 0.0 AxisValue) false false))

(event `InputAction|Fire`
  (params (Key :type "Key Structure"))
  (:`Pressed`
    (`TankAimingComponent.Fire` (`self.TankAiming`))))

(event `InputAxis|Left Track Throttle`
  (params (AxisValue :type "Float (single-precision)"))
  (`TankTrack.SetThrottle` (`self.TankTrack_L`) AxisValue))

(event `InputAxis|Right Track Throttle`
  (params (AxisValue :type "Float (single-precision)"))
  (`TankTrack.SetThrottle` (`self.TankTrack_R`) AxisValue))

(event `InputAxis|Forward_Intent`
  (params (AxisValue :type "Float (single-precision)"))
  (`TankMovementComponent.IntendMoveForward` (`self.TankMovement`) AxisValue))

(event `InputAxis|Right_Intent`
  (params (AxisValue :type "Float (single-precision)"))
  (`TankMovementComponent.IntendTurnRight` (`self.TankMovement`) AxisValue))

(fn `UserConstructionScript`)